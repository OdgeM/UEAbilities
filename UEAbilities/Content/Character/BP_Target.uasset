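; BP_Target is a targetable actor that displays stat bars and a team label through two widgets.
; On BeginPlay it binds its StatComponent to the StatBars widget and sets the Label text to its team name.
; Each Tick it scans the component's TickingStats and shows the stat bars only while the actor is targeted or any ticking value is above zero.
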(event `self.ReceiveBeginPlay`
  (bind _asstat_bars (cast `/Game/UI/StatBars` (`WidgetComponent.GetWidget` (`self.Widget`))))
  (set `/Game/UI/StatBars.Stat` (`self.StatComponent`) _asstat_bars)
  (set `/Game/UI/StatBars.Initialised` true _asstat_bars)
  (bind _aslabel (cast `/Game/UI/Label` (`WidgetComponent.GetWidget` (`self.Widget1`))))
  (`/Game/UI/Label.SetText` _aslabel (`|GetEnumeratorNameAsString` (`Targetable.GetTeam`))))

(event `self.ReceiveTick`
  (params (DeltaSeconds :type "Float (single-precision)"))
  (bind _tickingstats (`StatComponent.TickingStats` (`self.StatComponent`)))
  (bind _output_get (set `self.IsTicking` false))
  (bind _keys (`BlueprintMapLibrary.Map_Keys` _tickingstats))
  (for _array_element _keys
    (bind (_value _returnvalue) (`BlueprintMapLibrary.Map_Find` _tickingstats _array_element))
    (if _returnvalue
      (if (> _value 0)
        (set `self.IsTicking` true)
        (break))))
  (`SceneComponent.SetVisibility` (`self.Widget`) (or (`self.bIsTargeted`) _output_get) true))

(fn `UserConstructionScript`)